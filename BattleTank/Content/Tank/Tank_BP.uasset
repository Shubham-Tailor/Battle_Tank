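; Player-controllable tank Blueprint that wires turret, barrel, tracks and movement component to input.
; BeginPlay passes the turret and barrel references to the tank and initializes TankMovement with both tracks.
; Throttle axes drive each track directly, while move and turn axes send intents to TankMovement.
; Aim axes rotate the azimuth gimbal and spring arm separately, and the Fire action calls Fire.
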(event EventBeginPlay
  (Class|Tank|SetTurretReference (Variables|Default|GetTurret))
  (Class|Tank|SetBarrelReference (Variables|Default|GetBarrel))
  (Class|TankMovementComponent|Initialize (Variables|Default|GetTankMovement) (Variables|Default|GetTrack_left) (Variables|Default|GetTrack_Right)))

(event Input|ActionEvents|InputActionFire
  (params (Key :type Key%20Structure :default "None"))
  ;[1 1 1] input binding
  (:Pressed
    (Class|Tank|Fire)))

(event Input|AxisEvents|InputAxisAimAzimuth
  (params (AxisValue :type Float%20%28single-precision%29))
  ;[1 1 1] input binding
  (Transformation|AddLocalRotation (Variables|Default|GetAzimuthGimbal) (Math|Rotator|MakeRotator 0.0 0.0 AxisValue) false false))

(event Input|AxisEvents|InputAxisAimElevation
  (params (AxisValue :type Float%20%28single-precision%29))
  ;[1 1 1] input binding
  (Transformation|AddLocalRotation (Variables|Default|GetSpringArm) (Math|Rotator|MakeRotator 0.0 AxisValue 0.0) false false))

(event Input|AxisEvents|InputAxisLeftTrackThrottle
  (params (AxisValue :type Float%20%28single-precision%29))
  ;[1 1 1] Tank Throttle
  (Class|TankTrack|SetThrottle (Variables|Default|GetTrack_left) AxisValue))

(event Input|AxisEvents|InputAxisRightTrackThrottle
  (params (AxisValue :type Float%20%28single-precision%29))
  ;[1 1 1] Tank Throttle
  (Class|TankTrack|SetThrottle (Variables|Default|GetTrack_Right) AxisValue))

(event Input|AxisEvents|InputAxisMoveForward
  (params (AxisValue :type Float%20%28single-precision%29))
  ;[1 1 1] Tank Throttle
  (Class|TankMovementComponent|IntendMoveForward (Variables|Default|GetTankMovement) AxisValue))

(event Input|AxisEvents|InputAxisTurnRight
  (params (AxisValue :type Float%20%28single-precision%29))
  ;[1 1 1] Tank Throttle
  (Class|TankMovementComponent|IntendTurnRight (Variables|Default|GetTankMovement) AxisValue))

(fn ConstructionScript)